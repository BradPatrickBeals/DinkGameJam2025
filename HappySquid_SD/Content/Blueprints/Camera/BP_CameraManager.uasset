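; BP_CameraManager switches the first player controller's view between follow cameras, camera points and the player character.
; On BeginPlay it caches a BP_FollowCameraComponent actor and all camera points, then views through that camera.
; Space targets the Player reference, though FindPlayerCharacter, which fills it, is never called here.
; SwitchToStationary targets the follow-camera child actor of a given camera point.
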(event `self.ReceiveBeginPlay`
  (`self.FindPlayerCamera`)
  (`self.FindAllCameraPoints`)
  (`self.SetLocalCameraToViewCamera`))

(event `Key|SpaceBar`
  (params (Key :type "Key Structure"))
  (:`Pressed`
    (`self.SwitchToFollowPlayer`)))

(fn `FindAllCameraPoints`
  (bind _outactors (`GameplayStatics.GetAllActorsOfClass` "/Game/Blueprints/Camera/BP_CameraPoint.BP_CameraPoint_C"))
  (set `self.CameraPoints` _outactors))

(fn `FindPlayerCamera`
  (bind _returnvalue (`GameplayStatics.GetActorOfClass` "/Game/Blueprints/Camera/BP_FollowCameraComponent.BP_FollowCameraComponent_C"))
  (set `self.PlayerCamera` _returnvalue))

(fn `FindPlayerCharacter`
  (bind _returnvalue (`GameplayStatics.GetActorOfClass` "/Game/Blueprints/BP_PlayerCharacter.BP_PlayerCharacter_C"))
  (set `self.Player` _returnvalue)
  (return))

(fn `SetLocalCameraToViewCamera`
  (`/Engine/EditorBlueprintResources/StandardMacros.IsValid` (`self.PlayerCamera`)
    (:`Is Valid`
      _)
    (:`Is Not Valid`
      (`self.FindPlayerCamera`)))
  (`PlayerController.SetViewTargetWithBlend` (`GameplayStatics.GetPlayerController` 0) (`self.PlayerCamera`) 0.0 "VTBlend_Linear" 0.0 false)
  (return))

(fn `SwitchToFollowPlayer`
  (`PlayerController.SetViewTargetWithBlend` (`GameplayStatics.GetPlayerController` 0) (`self.Player`) 0.0 "VTBlend_Linear" 0.0 false))

(fn `SwitchToStationary`
  (params (`Camera Point` :type "/Game/Blueprints/Camera/BP_CameraPoint Object Reference"))
  (bind _asbp_follow_camera_component (cast `/Game/Blueprints/Camera/BP_FollowCameraComponent` (`ChildActorComponent.ChildActor` (`/Game/Blueprints/Camera/BP_CameraPoint.BP_FollowCameraComponent` `Camera Point`))))
  (`PlayerController.SetViewTargetWithBlend` (`GameplayStatics.GetPlayerController` 0) _asbp_follow_camera_component 0.0 "VTBlend_Linear" 0.0 false)
  (return))

(fn `UserConstructionScript`)