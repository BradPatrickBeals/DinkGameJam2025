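; Fan hazard manager that cycles through a list of fans, running one at a time in sequence.
; On BeginPlay it turns on each fan in FanList with its wind VFX for a fixed delay, then turns it off and moves to the next.
; After the last fan, a short pause restarts the sequence from the first, looping indefinitely.
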(event `self.ReceiveBeginPlay`
  (bind _fanlist (`self.FanList`))
  (bind _output_get (set `self.CurrentIndex` 0 :!label _label))
  (if (< _output_get (`KismetArrayLibrary.Array_Length` _fanlist)) :!label _label_2
    (bind _output (`|GetArrayItem` _fanlist _output_get))
    (set `/Game/Blueprints/Hazards/Fans/BP_Fan.IsActive` true _output)
    (`/Game/Blueprints/Hazards/Fans/BP_Fan.ToggleWindVFX` _output)
    (`/Game/Blueprints/Hazards/Fans/BP_Fan.ActivateFan` _output)
    (`KismetSystemLibrary.Delay` 2.0)
    (set `/Game/Blueprints/Hazards/Fans/BP_Fan.IsActive` false _output)
    (`/Game/Blueprints/Hazards/Fans/BP_Fan.ToggleWindVFX` _output)
    (`/Game/Blueprints/Hazards/Fans/BP_Fan.DeactivateFan` _output)
    (`/Engine/EditorBlueprintResources/StandardMacros.IncrementInt` _output_get
      (:`  `
        (goto _label_2)))
    (else
      (`KismetSystemLibrary.Delay` 0.1)
      (goto _label))))

(fn `UserConstructionScript`)