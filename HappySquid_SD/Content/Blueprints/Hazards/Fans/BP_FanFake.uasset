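; BP_FanFake is a fan hazard that spins visually and launches whatever enters its Box trigger.
; A looping timer started at BeginPlay yaws the Fans component by CurrentSpeed, in place of Tick.
; On overlap, physics-simulating components get a mass-independent impulse along the actor's forward vector scaled by LaunchForce.
; Otherwise, Characters are launched straight up at a fixed velocity, regardless of fan orientation or LaunchForce.
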(event `SpinTick`
  ; Rotation setup and calling Custom material
  (`SceneComponent.K2_AddLocalRotation` (`self.Fans`) (`KismetMathLibrary.MakeRotator` 0.0 0.0 (* (`self.CurrentSpeed`) 0.01)) false false))

(event `self.ReceiveBeginPlay`
  ; Rotation setup and calling Custom material
  (`KismetSystemLibrary.K2_SetTimerDelegate` (delegate `SpinTick`) 0.01 true))

(event `self.Box.OnComponentBeginOverlap`
  (params (OverlappedComponent :type "PrimitiveComponent Object Reference") (OtherActor :type "Actor Object Reference") (OtherComp :type "PrimitiveComponent Object Reference") (OtherBodyIndex :type Integer) (bFromSweep :type Boolean) (SweepResult :type "HitResult Structure (by ref)"))
  (if true
    (if (`SceneComponent.IsSimulatingPhysics` OtherComp "None")
      (`PrimitiveComponent.AddImpulse` OtherComp (* (`self.GetActorForwardVector`) (`self.LaunchForce`)) "None" true)
      (else
        (bind _ascharacter (cast `Character` OtherActor))
        (`Character.LaunchCharacter` _ascharacter (0.0 0.0 900.0) false true)))))

(fn `UserConstructionScript`)