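; BP_FanManager is a hazard manager that cycles the level's BP_Fan actors so they blow one at a time.
; On BeginPlay it gathers every BP_Fan into FanList, printing a warning if none are found.
; A latent Delay loop activates each fan with its wind VFX for two seconds, switches it off, then advances, restarting after a brief pause at the list's end.
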(event `self.ReceiveBeginPlay`
  (bind _fanlist (`self.FanList`))
  (bind _outactors (`GameplayStatics.GetAllActorsOfClass` "/Game/Blueprints/Hazards/Fans/BP_Fan.BP_Fan_C"))
  (bind _output_get (set `self.FanList` _outactors))
  (if (== (`KismetArrayLibrary.Array_Length` _output_get) 0)
    (`KismetSystemLibrary.PrintString` "No Fans Assigned to Manager -- BP_FanManager -- Event BeginPlay")
    (else
      (bind _output_get_2 (set `self.CurrentIndex` 0 :!label _label))
      (if (< _output_get_2 (`KismetArrayLibrary.Array_Length` _fanlist)) :!label _label_2
        (bind _output (`|GetArrayItem` _fanlist _output_get_2))
        (set `/Game/Blueprints/Hazards/Fans/BP_Fan.IsActive` true _output)
        (`/Game/Blueprints/Hazards/Fans/BP_Fan.ToggleWindVFX` _output)
        (`/Game/Blueprints/Hazards/Fans/BP_Fan.ActivateFan` _output)
        (`KismetSystemLibrary.Delay` 2.0)
        (set `/Game/Blueprints/Hazards/Fans/BP_Fan.IsActive` false _output)
        (`/Game/Blueprints/Hazards/Fans/BP_Fan.ToggleWindVFX` _output)
        (`/Game/Blueprints/Hazards/Fans/BP_Fan.DeactivateFan` _output)
        (`/Engine/EditorBlueprintResources/StandardMacros.IncrementInt` _output_get_2
          (:`  `
            (goto _label_2)))
        (else
          (`KismetSystemLibrary.Delay` 0.1)
          (goto _label))))))

(fn `UserConstructionScript`)