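; BP_Sprinkle is a short-lived physics sprinkle, tinted by its SprinkleColor through a dynamic material.
; On BeginPlay it launches itself with a random upward cone impulse, applied as a velocity change.
; After a randomized delay it disables collision, spawns a Niagara vapor effect at the mesh and runs a timeline driving the material's dissolve parameter.
; The graph does not destroy the actor once the dissolve finishes.
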(event `self.ReceiveBeginPlay`
  (bind _staticmesh (`self.StaticMesh`))
  (bind _returnvalue (`PrimitiveComponent.CreateDynamicMaterialInstance` _staticmesh 0 null "None"))
  (`MaterialInstanceDynamic.SetVectorParameterValue` _returnvalue "BaseColor" (`self.SprinkleColor`))
  (`PrimitiveComponent.AddImpulse` _staticmesh (* (`KismetMathLibrary.RandomUnitVectorInConeInDegrees` (0.0 0.0 1.0) 45.0) (`KismetMathLibrary.RandomFloatInRange` 300.0 600.0)) "None" true)
  (`KismetSystemLibrary.Delay` (`KismetMathLibrary.RandomFloatInRange` 10.0 13.0))
  (`PrimitiveComponent.SetCollisionEnabled` _staticmesh "NoCollision")
  (`NiagaraFunctionLibrary.SpawnSystemAtLocation` "/Game/VFX/NS_SprinkleVapor.NS_SprinkleVapor" (`SceneComponent.K2_GetComponentLocation` _staticmesh))
  (bind (_direction _alpha) (`Timeline|Dissolve Timeline` :!via `PlayFromStart`)
    (:`Update`
      (`MaterialInstanceDynamic.SetScalarParameterValue` _returnvalue "dissolveAlpha" _alpha))))

(fn `UserConstructionScript`)