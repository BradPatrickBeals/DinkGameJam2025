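; Player controller that prepares a local player for gameplay and holds a reference to the level's BP_CameraManager.
; On BeginPlay, only for the local controller, it switches to game-only input, hides the mouse cursor, clears all widgets and caches the camera manager actor by class.
; FindCameraManager repeats that lookup as a standalone function, while the Possess event is empty.
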(event `self.ReceiveBeginPlay`
  (if (`self.IsLocalPlayerController`)
    (`WidgetBlueprintLibrary.SetInputMode_GameOnly` self)
    (set `self.bShowMouseCursor` false)
    (`WidgetLayoutLibrary.RemoveAllWidgets`)
    (bind _returnvalue (`GameplayStatics.GetActorOfClass` "/Game/Blueprints/Camera/BP_CameraManager.BP_CameraManager_C"))
    (set `self.Camera Manager` _returnvalue)))

(event `self.ReceivePossess`
  (params (PossessedPawn :type "Pawn Object Reference")))

(fn `FindCameraManager`
  (bind _returnvalue (`GameplayStatics.GetActorOfClass` "/Game/Blueprints/Camera/BP_CameraManager.BP_CameraManager_C"))
  (set `self.Camera Manager` _returnvalue)
  (return))

(fn `UserConstructionScript`)