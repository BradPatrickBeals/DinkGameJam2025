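; Small conveyor belt actor that pushes characters and physics objects horizontally along its negative right vector.
; Box overlap events track physics-simulating components and character components, removing them when overlap ends.
; Each Tick launches characters with an additive, delta-scaled velocity and applies mass-independent acceleration to other components, both scaled by Speed with separate multipliers.
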(event `self.Box.OnComponentBeginOverlap`
  (params (OverlappedComponent :type "PrimitiveComponent Object Reference") (OtherActor :type "Actor Object Reference") (OtherComp :type "PrimitiveComponent Object Reference") (OtherBodyIndex :type Integer) (bFromSweep :type Boolean) (SweepResult :type "HitResult Structure (by ref)"))
  (if (`SceneComponent.IsSimulatingPhysics` OtherComp "None")
    (`KismetArrayLibrary.Array_Add` (`self.OverLappingComponents`) OtherComp)
    (else
      (cast `Character` OtherActor)
      (`KismetArrayLibrary.Array_Add` (`self.OverLappingComponents`) OtherComp))))

(event `self.ReceiveTick`
  (params (DeltaSeconds :type "Float (single-precision)"))
  (bind _returnvalue (* (`self.GetActorRightVector`) (-1.0 -1.0 0.0)))
  (for _array_element (`self.OverLappingComponents`)
    (bind _ascharacter (cast `Character` (`ActorComponent.GetOwner` _array_element))
      (:`then`
        (`Character.LaunchCharacter` _ascharacter (* (* _returnvalue (`self.Speed`)) DeltaSeconds 8.0) false false))
      (:`CastFailed`
        (`PrimitiveComponent.AddForce` _array_element (* _returnvalue (`self.Speed`) 2.0) "None" true)))))

(event `self.Box.OnComponentEndOverlap`
  (params (OverlappedComponent :type "PrimitiveComponent Object Reference") (OtherActor :type "Actor Object Reference") (OtherComp :type "PrimitiveComponent Object Reference") (OtherBodyIndex :type Integer))
  (`KismetArrayLibrary.Array_RemoveItem` (`self.OverLappingComponents`) OtherComp))

(fn `UserConstructionScript`)