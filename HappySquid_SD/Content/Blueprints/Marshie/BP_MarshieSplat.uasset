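; BP_MarshieSplat is a short-lived physics sprinkle, tinted with SprinkleColor and launched along LaunchDirection with slight random spread and speed on BeginPlay.
; After a random delay it disables collision, spawns a vapor Niagara effect and runs a timeline that dissolves its dynamic material before destroying itself.
; The kicked and falling sound logic is disconnected from the empty hit event, so it never runs.
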(event `self.ReceiveBeginPlay`
  (bind _staticmesh (`self.StaticMesh`))
  (bind _returnvalue (`PrimitiveComponent.CreateDynamicMaterialInstance` _staticmesh 0 null "None"))
  (`MaterialInstanceDynamic.SetVectorParameterValue` _returnvalue "BaseColor" (`self.SprinkleColor`))
  (`PrimitiveComponent.AddImpulse` _staticmesh (* (`KismetMathLibrary.RandomUnitVectorInConeInDegrees` (`self.LaunchDirection`) 2.0) (`KismetMathLibrary.RandomFloatInRange` 1200.0 1800.0)) "None" true)
  (`KismetSystemLibrary.Delay` (`KismetMathLibrary.RandomFloatInRange` 10.0 13.0))
  (`PrimitiveComponent.SetCollisionEnabled` _staticmesh "NoCollision")
  (`NiagaraFunctionLibrary.SpawnSystemAtLocation` "/Game/VFX/NS_SprinkleVapor.NS_SprinkleVapor" (`SceneComponent.K2_GetComponentLocation` _staticmesh))
  (bind (_direction _alpha) (`Timeline|Dissolve Timeline` :!via `PlayFromStart`)
    (:`Update`
      (`MaterialInstanceDynamic.SetScalarParameterValue` _returnvalue "dissolveAlpha" _alpha))
    (:`Finished`
      (`self.K2_DestroyActor`))))

(event `self.StaticMesh.OnComponentHit`
  (params (HitComponent :type "PrimitiveComponent Object Reference") (OtherActor :type "Actor Object Reference") (OtherComp :type "PrimitiveComponent Object Reference") (NormalImpulse :type "Vector Structure") (Hit :type "HitResult Structure (by ref)"))
  ;[0.01453 0.15 0 0.5] Sprinkle Sound
)

(fn `UserConstructionScript`)