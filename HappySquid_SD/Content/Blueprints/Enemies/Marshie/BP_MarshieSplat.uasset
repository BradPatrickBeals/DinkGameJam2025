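; BP_MarshieSplat is a short-lived, colored sprinkle piece that scatters from a Marshie enemy as physics debris.
; On BeginPlay it tints a dynamic material with SprinkleColor and launches Blob1 in a random cone around LaunchDirection.
; After a randomized delay it switches to query-only collision, spawns a vapor Niagara effect, and runs a dissolve timeline before destroying itself.
; The component-hit event is empty, leaving its kicked and falling sprinkle sounds disconnected.
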(event `self.ReceiveBeginPlay`
  (bind _blob_1 (`self.Blob 1`))
  (bind _returnvalue (`PrimitiveComponent.CreateDynamicMaterialInstance` _blob_1 0 null "None"))
  (`MaterialInstanceDynamic.SetVectorParameterValue` _returnvalue "BaseColor" (`self.SprinkleColor`))
  (`PrimitiveComponent.AddImpulse` _blob_1 (* (`KismetMathLibrary.RandomUnitVectorInConeInDegrees` (`self.LaunchDirection`) 20.0) (`KismetMathLibrary.RandomFloatInRange` 400.0 600.0)) "None" true)
  (`KismetSystemLibrary.Delay` (`KismetMathLibrary.RandomFloatInRange` 10.0 13.0))
  (`PrimitiveComponent.SetCollisionEnabled` _blob_1 "QueryOnly")
  (`NiagaraFunctionLibrary.SpawnSystemAtLocation` "/Game/VFX/NS_SprinkleVapor.NS_SprinkleVapor" (`SceneComponent.K2_GetComponentLocation` _blob_1))
  (bind (_direction _alpha) (`Timeline|Dissolve Timeline` :!via `PlayFromStart`)
    (:`Update`
      (`MaterialInstanceDynamic.SetScalarParameterValue` _returnvalue "dissolveAlpha" _alpha))
    (:`Finished`
      (`self.K2_DestroyActor`))))

(event `self.Blob 1.OnComponentHit`
  (params (HitComponent :type "PrimitiveComponent Object Reference") (OtherActor :type "Actor Object Reference") (OtherComp :type "PrimitiveComponent Object Reference") (NormalImpulse :type "Vector Structure") (Hit :type "HitResult Structure (by ref)"))
  ;[0.01453 0.15 0 0.5] Sprinkle Sound
)

(fn `UserConstructionScript`)