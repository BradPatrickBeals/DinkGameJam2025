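; BP_Sprinkle is an enemy-folder actor (Marshie) that bursts into colored sprinkles when whacked by the player character.
; GetWhacked spawns twenty more BP_Sprinkle actors at its location, launched away from the attacker with a slight upward bias, and sets its StaticMesh to ignore PhysicsBody collision.
; Each gets a random palette color, though the random range reaches only the first four of six options.
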(event `GetWhacked`
  (params (Attacker :type "Actor Object Reference"))
  (bind _returnvalue (`self.K2_GetActorLocation`))
  (cast `/Game/Blueprints/BP_PlayerCharacter` Attacker)
  (for _ (range 1 21)
    (`|SpawnActorFromClass` "/Game/Blueprints/BP_Sprinkle.BP_Sprinkle_C" (`KismetMathLibrary.MakeTransform` _returnvalue) "AlwaysSpawn" "MultiplyWithRoot" null (select `int` (`KismetMathLibrary.RandomIntegerInRange` 0 3) :`0` (struct :`R` 1.0 :`G` 0.01257 :`B` 0.802794 :`A` 1.0) :`1` (struct :`G` 0.034036 :`B` 1.0 :`A` 1.0) :`2` (struct :`R` 1.0 :`B` 0.049463 :`A` 1.0) :`3` (struct :`R` 1.0 :`G` 0.840906 :`A` 1.0) :`4` (struct :`R` 1.0 :`G` 1.0 :`B` 1.0 :`A` 1.0) :`5` (struct :`R` 0.191264 :`G` 1.0 :`A` 1.0) :!type "LinearColor Structure") (+ (`KismetMathLibrary.Normal` (- _returnvalue (`self.K2_GetActorLocation` Attacker))) (0.0 0.0 0.02)) null)
    (`PrimitiveComponent.SetCollisionResponseToChannel` (`self.StaticMesh`) "ECC_PhysicsBody" "ECR_Ignore")))

(fn `UserConstructionScript`)