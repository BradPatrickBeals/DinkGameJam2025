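; BP_SweetDecietMenu_GameMode is the menu game mode that manages the player list for the multiplayer lobby.
; In Lvl Lobby Menu, new players' menu controllers are tracked and told to create the lobby UI and run initial setup.
; UpdateLobby rebuilds profiles from tracked controllers and pushes names or the selected level to each one.
; Logout removes the leaving controller and refreshes the names for remaining players.
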(event `self.K2_OnLogout`
  (params (ExitingController :type "Controller Object Reference"))
  (bind _asbp_sweet_deciet_menu_controller (cast `/Game/Framework/BP_SweetDecietMenuController` ExitingController))
  (`KismetArrayLibrary.Array_RemoveItem` (`self.All_ConnectedPlayers`) _asbp_sweet_deciet_menu_controller)
  (`self.UpdateLobby` true))

(event `self.HandleStartingNewPlayer`
  (params (NewPlayer :type "PlayerController Object Reference"))
  (bind _returnvalue (`GameplayStatics.GetCurrentLevelName` true))
  (switch `string` _returnvalue
    (:`Lvl_LobbyMenu`
      (bind _asbp_sweet_deciet_menu_controller (cast `/Game/Framework/BP_SweetDecietMenuController` NewPlayer))
      (`KismetArrayLibrary.Array_Add` (`self.All_ConnectedPlayers`) _asbp_sweet_deciet_menu_controller)
      (`/Game/Framework/BP_SweetDecietMenuController.CreateLobbyMenu` _asbp_sweet_deciet_menu_controller)
      (`/Game/Framework/BP_SweetDecietMenuController.Initial_Setup` _asbp_sweet_deciet_menu_controller))))

(event `UpdateLobby`
  (params (`Player Names` :type Boolean) (LevelSelection :type Boolean))
  (if `Player Names`
    (`KismetArrayLibrary.Array_Clear` (`self.All_PlayerProfiles`))
    (for _array_element (`self.All_ConnectedPlayers`)
      (`KismetArrayLibrary.Array_Add` (`self.All_PlayerProfiles`) (`/Game/Framework/BP_SweetDecietMenuController.Player Profile Info` _array_element))))
  (for _array_element_2 (`self.All_ConnectedPlayers`)
    (if `Player Names`
      (`/Game/Framework/BP_SweetDecietMenuController.UpdatePlayerNames` _array_element_2 (`self.All_PlayerProfiles`)))
    (if LevelSelection
      (`/Game/Framework/BP_SweetDecietMenuController.UpdateLevelSelection` _array_element_2 (`self.SelectedLevelName`)))))

(fn `UserConstructionScript`)