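; Game instance for SweetDeciet that handles the main menu, solo game start and player profile persistence.
; UIShowMainMenu creates WB_MainMenu once, then displays it with UI-only input and a visible cursor.
; CheckForSavedProfile loads the SG_PlayerProfile save slot if it exists, otherwise saves the current PlayerProfileInfo into it.
; Start_SoloGame sets IsSoloGame to false, despite its name, and opens the Welcome_to_the_floor level.
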(event `Start_SoloGame`
  (set `self.IsSoloGame` false)
  (`GameplayStatics.OpenLevelBySoftObjectPtr` "/Game/Levels/Zone_One/Welcome_to_the_floor/Welcome_to_the_floor.Welcome_to_the_floor"))

(fn `CheckForSavedProfile`
  (bind _returnvalue (`GameplayStatics.DoesSaveGameExist` (`self.Player Profile Slot`)))
  (if _returnvalue
    (`self.LoadProfile`)
    (else
      (`self.SaveProfile`)))
  (return))

(fn `LoadProfile`
  (bind _returnvalue (`GameplayStatics.LoadGameFromSlot` (`self.Player Profile Slot`)))
  (bind _assg_player_profile (cast `/Game/SaveData/SG_PlayerProfile` _returnvalue))
  (set `self.Player Profile Info` (`/Game/SaveData/SG_PlayerProfile.PlayerProfile` _assg_player_profile))
  (return))

(fn `SaveProfile`
  (bind _sg_player_profile (`self.SG Player Profile`))
  (`/Engine/EditorBlueprintResources/StandardMacros.IsValid` (`self.SG Player Profile`)
    (:`Is Valid`
      _)
    (:`Is Not Valid`
      (bind _returnvalue (`GameplayStatics.CreateSaveGameObject` "/Game/SaveData/SG_PlayerProfile.SG_PlayerProfile_C"))
      (set `self.SG Player Profile` _returnvalue)))
  (set `/Game/SaveData/SG_PlayerProfile.PlayerProfile` (`self.Player Profile Info`) _sg_player_profile)
  (`GameplayStatics.SaveGameToSlot` _sg_player_profile (`self.Player Profile Slot`))
  (return))

(fn `UI_ShowMainMenu`
  (bind _returnvalue (`GameplayStatics.GetPlayerController` 0))
  (bind _wb_mainmenu (`self.WB_MainMenu`))
  (`/Engine/EditorBlueprintResources/StandardMacros.IsValid` (`self.WB_MainMenu`)
    (:`Is Valid`
      _)
    (:`Is Not Valid`
      (bind _returnvalue_2 (`|CreateWidget` "/Game/Blueprints/MainMenu/WB_MainMenu.WB_MainMenu_C" _returnvalue))
      (set `self.WB_MainMenu` _returnvalue_2)))
  (`UserWidget.AddToViewport` _wb_mainmenu 0)
  (`WidgetBlueprintLibrary.SetInputMode_UIOnlyEx` _returnvalue _wb_mainmenu)
  (set `PlayerController.bShowMouseCursor` true _returnvalue)
  (return))