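; Player controller for the main menu, handling menu input, the lobby screen and leaving a session.
; On BeginPlay, the local controller shows the mouse cursor and switches to UI-only input.
; CreateLobbyMenu creates the WB_LobbyMenu widget on first use, caches it and adds it to the viewport.
; EndClientSession calls DestroySession and opens Lvl_Menu from its immediate exec pin, without waiting for success or failure.
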(event `self.ReceiveBeginPlay`
  (if (`self.IsLocalController`)
    (set `self.bShowMouseCursor` true)
    (`WidgetBlueprintLibrary.SetInputMode_UIOnlyEx` self null)))

(event `EndClientSession`
  (`DestroySessionCallbackProxy.DestroySession` self
    (:`then`
      (`GameplayStatics.OpenLevelBySoftObjectPtr` "/Game/Levels/Menu/Lvl_Menu.Lvl_Menu"))))

(event `CreateLobbyMenu`
  (`self.UI_ShowLobbyMenu`))

(fn `UI_ShowLobbyMenu`
  (`/Engine/EditorBlueprintResources/StandardMacros.IsValid` (`self.WB_LobbyMenu`)
    (:`Is Valid`
      _)
    (:`Is Not Valid`
      (bind _returnvalue (`|GenericCreateObject` (`GameplayStatics.GetPlayerController` 0) "/Game/Blueprints/MainMenu/UI/WB_LobbyMenu.WB_LobbyMenu_C"))
      (set `self.WB_LobbyMenu` _returnvalue)))
  (`UserWidget.AddToViewport` (`self.WB_LobbyMenu`) 0)
  (return))

(fn `UserConstructionScript`)