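; BP_Spawner spawns BP_EnemyCharacter enemies at its own transform while limiting their world-wide population.
; It spawns on BeginPlay, then retries whenever a countdown from SpawnTime expires, decremented once per Tick, so timing depends on frame rate.
; Each attempt counts all living or present enemy actors: at or below SpawnMinimum it always spawns, otherwise a coin flip decides, provided the count is below SpawnLimit.
; Each valid new enemy receives OnSpawn.
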(event `self.ReceiveBeginPlay`
  (`self.Spawn`)
  (set `self.Interval` (`self.SpawnTime`)))

(event `self.ReceiveTick`
  (params (DeltaSeconds :type "Float (single-precision)"))
  (bind _result (`/Engine/EditorBlueprintResources/StandardMacros.DecrementFloat` (`self.Interval`))
    (:`  `
      (bind _output_get (set `self.Interval` _result))
      (if (<= _output_get 0.0)
        (`self.Spawn`)
        (set `self.Interval` (`self.SpawnTime`))))))

(event `Spawn`
  (bind _outactors (`GameplayStatics.GetAllActorsOfClass` "/Game/Blueprints/BP_EnemyCharacter.BP_EnemyCharacter_C"))
  (bind _returnvalue (`KismetArrayLibrary.Array_Length` _outactors))
  (if (< _returnvalue (`self.Spawn Limit`))
    (if (<= _returnvalue (`self.Spawn Minimum`))
      (bind _returnvalue_2 (`|SpawnActorFromClass` "/Game/Blueprints/BP_EnemyCharacter.BP_EnemyCharacter_C" (`self.GetTransform`) "Undefined" "MultiplyWithRoot" null null :!label _label))
      (if (`KismetSystemLibrary.IsValid` _returnvalue_2)
        (`/Game/Blueprints/BP_EnemyCharacter.OnSpawn` _returnvalue_2))
      (elif (== (`KismetMathLibrary.RandomIntegerInRange` 1 2) 1)
        (goto _label)))))

(fn `UserConstructionScript`)