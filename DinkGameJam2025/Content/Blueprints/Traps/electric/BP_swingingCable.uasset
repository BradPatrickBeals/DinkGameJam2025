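; Swinging electric cable trap that briefly freezes the player on contact.
; On BeginPlay a Timeline drives the cable Cylinder's world roll and pitch, scaled by the X and Y variables to set the swing direction, with yaw held at zero.
; When BP_PlayerCharacter overlaps the Box, its movement mode is set to None, then restored to Walking after a half-second delay.
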(event `self.ReceiveBeginPlay`
  (bind (_direction _newtrack_0) (`Timeline|Timeline`)
    (:`Update`
      (`SceneComponent.K2_SetWorldRotation` (`self.Cylinder`) (`KismetMathLibrary.MakeRotator` (* _newtrack_0 (`self.x`)) (* _newtrack_0 (`self.y`))) false false))))

(event `self.Box.OnComponentBeginOverlap`
  (params (OverlappedComponent :type "PrimitiveComponent Object Reference") (OtherActor :type "Actor Object Reference") (OtherComp :type "PrimitiveComponent Object Reference") (OtherBodyIndex :type Integer) (bFromSweep :type Boolean) (SweepResult :type "HitResult Structure (by ref)"))
  (bind _asbp_third_person_character (cast `/Game/Blueprints/BP_PlayerCharacter` OtherActor))
  (bind _charactermovement (`Character.CharacterMovement` _asbp_third_person_character))
  (`CharacterMovementComponent.SetMovementMode` _charactermovement "MOVE_None" 0)
  (`KismetSystemLibrary.Delay` 0.5)
  (`CharacterMovementComponent.SetMovementMode` _charactermovement "MOVE_Walking" 0))

(fn `UserConstructionScript`)